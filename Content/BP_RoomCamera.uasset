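; BP_RoomCamera is a room camera actor that becomes the view target when a TopDownCharacter enters its Box trigger.
; On overlap, it gets that character's TopDownController and blends the view to itself over a short transition.
; A ForceSetCam event applies the same blend to the first player's controller without needing an overlap.
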(event `ForceSetCam`
  (`PlayerController.SetViewTargetWithBlend` (cast `/Game/TopDownBP/Blueprints/TopDownController` (`Pawn.GetController` (`GameplayStatics.GetPlayerCharacter` 0)) :!pure true) self 0.2 "VTBlend_Linear" 0.0 false))

(event `self.Box.OnComponentBeginOverlap`
  (params (OverlappedComponent :type "PrimitiveComponent Object Reference") (OtherActor :type "Actor Object Reference") (OtherComp :type "PrimitiveComponent Object Reference") (OtherBodyIndex :type Integer) (bFromSweep :type Boolean) (SweepResult :type "HitResult Structure (by ref)"))
  (bind _astop_down_character (cast `/Game/TopDownBP/Blueprints/TopDownCharacter` OtherActor))
  (`PlayerController.SetViewTargetWithBlend` (cast `/Game/TopDownBP/Blueprints/TopDownController` (`Pawn.GetController` _astop_down_character) :!pure true) self 0.2 "VTBlend_Linear" 0.0 false))

(fn `UserConstructionScript`)