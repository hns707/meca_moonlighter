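; BP_Doors is a Blueprint that opens or closes four directional doors (N, S, E, O).
; BeginPlay collects the door components into an ordered array.
; SetDoors stores an array of open flags and applies it by index, hiding open doors and disabling their collision.
; Closed doors are made visible, but their collision is not re-enabled.
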(event `self.ReceiveBeginPlay`
  (bind _doors (`self.Doors`))
  (`KismetArrayLibrary.Array_Add` _doors (`self.N`))
  (`KismetArrayLibrary.Array_Add` _doors (`self.S`))
  (`KismetArrayLibrary.Array_Add` _doors (`self.E`))
  (`KismetArrayLibrary.Array_Add` _doors (`self.O`)))

(event `SetDoors`
  (params (`DoorsOpen?` :type "Array of Boolean"))
  (set `self.DoorsStatus` `DoorsOpen?`)
  (for (_array_element _array_index) (`self.Doors`)
    (bind _output (`|GetArrayItem` `DoorsOpen?` _array_index))
    (`SceneComponent.SetVisibility` _array_element (not _output) false)
    (if _output
      (`PrimitiveComponent.SetCollisionEnabled` _array_element "NoCollision"))))

(fn `UserConstructionScript`)